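; GM_Workers is the game mode for a worker test that tracks the gathered wood count.
; On BeginPlay it creates the WB_Main widget and adds it to the viewport.
; Its events add one wood or subtract a given amount, then tell the widget to refresh its wood count display.
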(event `self.ReceiveBeginPlay`
  (bind _returnvalue (`|CreateWidget` "/Game/TestWorkers/Blueprints/WB_Main.WB_Main_C"))
  (`UserWidget.AddToViewport` _returnvalue 0))

(event `AddGatheredWoodCount`
  (`/Engine/EditorBlueprintResources/StandardMacros.IncrementInt` (`self.GatheredWoodCount`)
    (:`  `
      (`/Game/TestWorkers/Blueprints/WB_Main.UpdateWoodCount` (stale `self.ReceiveBeginPlay` _returnvalue)))))

(event `SubtractGatheredWoodCount`
  (params (Amount :type Integer))
  (set `self.GatheredWoodCount` (- (`self.GatheredWoodCount`) Amount))
  (`/Game/TestWorkers/Blueprints/WB_Main.UpdateWoodCount` (stale `self.ReceiveBeginPlay` _returnvalue)))

(fn `UserConstructionScript`)